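; A laser hazard actor that casts a beam from one block toward another and damages what it hits.
; On BeginPlay it spawns a separate LaserBeam actor to draw the beam.
; Tick, followed by a short Delay, line-traces along LaserBlock1's forward vector for the distance to LaserBlock2, ending the beam at any blocking hit.
; Hit actors with a HealthComponent take point damage, limited by a shared cooldown timer.
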(event `self.ReceiveBeginPlay`
  (set `self.LastTimeDamage` (`self.DamageResetTimer`))
  (bind _returnvalue (`|SpawnActorFromClass` "/Game/Blueprints/LaserBeam.LaserBeam_C" (`self.GetTransform`) "Undefined" "OverrideRootScale" self null))
  (set `self.LaserBeamMesh` _returnvalue))

(event `self.ReceiveTick`
  (params (DeltaSeconds :type "Float (single-precision)"))
  (bind _laserblock1 (`self.LaserBlock1`))
  (bind _returnvalue (`SceneComponent.K2_GetComponentLocation` _laserblock1))
  (bind _returnvalue_2 (+ _returnvalue (* (`SceneComponent.GetForwardVector` _laserblock1) (`KismetMathLibrary.VSize` (- (`SceneComponent.K2_GetComponentLocation` (`self.LaserBlock2`)) (`SceneComponent.K2_GetComponentLocation` (`self.LaserBlock1`)))))))
  (set `self.LastTimeDamage` (+ (`self.LastTimeDamage`) (`GameplayStatics.GetWorldDeltaSeconds`)))
  (`KismetSystemLibrary.Delay` 0.01)
  (`|ExecutionSequence`
    (:`then_0`
      (bind (_outhit _returnvalue_3) (`KismetSystemLibrary.LineTraceSingle` _returnvalue _returnvalue_2 "TraceTypeQuery3" true (`|MakeArray` self (`self.LaserBeamMesh`) :!type "Actor Object Reference") "None" true (struct :`R` 1.0 :`A` 1.0) (struct :`G` 1.0 :`A` 1.0) 0.1))
      (set `self.BeamStart` (`SceneComponent.K2_GetComponentLocation` (`self.LaserBlock1`)))
      (if _returnvalue_3
        (bind (_bblockinghit _binitialoverlap _time _distance _location _impactpoint _normal _impactnormal _physmat _hitactor) (`GameplayStatics.BreakHitResult` _outhit))
        (set `self.BeamEnd` _impactpoint)
        (`/Engine/EditorBlueprintResources/StandardMacros.IsValid` (`self.GetComponentByClass` _hitactor "/Script/GMTKGameJam2020.HealthComponent")
          (:`Is Valid`
            (if (>= (`self.LastTimeDamage`) (`self.DamageResetTimer`))
              (`GameplayStatics.ApplyPointDamage` _hitactor (`self.LaserDamage`) _impactpoint (`GameplayStatics.MakeHitResult` false))
              (set `self.LastTimeDamage` 0.0))))
        (else
          (set `self.BeamEnd` _returnvalue_2))))
    (:`then_1`
      (`/Game/Blueprints/LaserBeam.SetBeam` (`self.LaserBeamMesh`) (`self.BeamStart`) (`self.BeamEnd`)))))

(fn `UserConstructionScript`)