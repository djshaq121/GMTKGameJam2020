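; Player Blueprint that sets up the player's HUD and handles death.
; On BeginPlay it creates the Player_UI widget bound to its Health component, switches to game-only input with a hidden cursor, and binds to the component's health-change event.
; When health reaches zero, it clears widgets, shows GameOver_UI with UI input and a visible cursor, disables input, plays a sound and destroys the actor.
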(event `self.ReceiveBeginPlay`
  (bind _returnvalue (`GameplayStatics.GetPlayerController` 0))
  (`|ExecutionSequence`
    (:`then_0`
      (bind _returnvalue_2 (`|CreateWidget` "/Game/UI/Player_UI.Player_UI_C" null (`self.Health`)))
      (`UserWidget.AddToViewport` _returnvalue_2 0)
      (`WidgetBlueprintLibrary.SetInputMode_GameOnly` _returnvalue)
      (`self.EnableInput` _returnvalue)
      (set `PlayerController.bShowMouseCursor` false _returnvalue))
    (:`then_1`
      (add `HealthComponent.OnHealthChange` (`self.Health`) (delegate `OnHealthChange_Event_0`)))))

(event `OnHealthChange_Event_0`
  (params (HealthComp :type "HealthComponent Object Reference") (Health :type "Float (double-precision)") (HealthChange :type "Float (double-precision)") (HitDirection :type "Vector Structure") (DamageType :type "DamageType Object Reference") (InstigatedBy :type "Controller Object Reference") (DamageCauser :type "Actor Object Reference"))
  (bind _returnvalue (`GameplayStatics.GetPlayerController` 0))
  (if (<= Health 0.0)
    (`|ExecutionSequence`
      (:`then_0`
        (`WidgetLayoutLibrary.RemoveAllWidgets`)
        (bind _returnvalue_2 (`|CreateWidget` "/Game/UI/GameOver_UI.GameOver_UI_C"))
        (`UserWidget.AddToViewport` _returnvalue_2 0)
        (`WidgetBlueprintLibrary.SetInputMode_GameAndUIEx` _returnvalue _returnvalue_2)
        (set `PlayerController.bShowMouseCursor` true _returnvalue)
        (`self.DisableInput` _returnvalue))
      (:`then_1`
        (`GameplayStatics.PlaySoundAtLocation` null (`self.K2_GetActorLocation`) (struct) 1.0 1.0 0.0 null null null)
        (`self.K2_DestroyActor`)))))

(fn `UserConstructionScript`)